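; BP_Player is the player Blueprint, which switches between flat-screen and VR display according to the current level.
; On BeginPlay it matches the level name: Menu disables the HMD and stereo rendering, then shows the UMG_MainMenu widget.
; Castle enables the HMD and stereo rendering.
; Tick is empty, and delayed level-switch chains between Castle and Menu are left unconnected, so they never run.
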(event `self.ReceiveBeginPlay`
  (bind _returnvalue (`GameplayStatics.GetPlayerController` 0))
  (bind _returnvalue_2 (`GameplayStatics.GetCurrentLevelName` true))
  (switch `string` _returnvalue_2
    (:`Menu`
      (`HeadMountedDisplayFunctionLibrary.EnableHMD` false)
      (`KismetSystemLibrary.ExecuteConsoleCommand` "stereo off" _returnvalue)
      (bind _returnvalue_3 (`|CreateWidget` "/Game/UI/Widget/UMG_MainMenu.UMG_MainMenu_C" _returnvalue))
      (`UserWidget.AddToViewport` _returnvalue_3 0))
    (:`Castle`
      (`HeadMountedDisplayFunctionLibrary.EnableHMD` true)
      (`KismetSystemLibrary.ExecuteConsoleCommand` "stereo on" (`GameplayStatics.GetPlayerController` 0)))))

(event `self.ReceiveTick`
  (params (DeltaSeconds :type "Float (single-precision)")))

(fn `UserConstructionScript`)