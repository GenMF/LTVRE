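; BP_Object is a quiz object with static meshes and separate question widgets for teacher, practice and student.
; Tick pushes its notice, question, answers and self-reference into all three widgets.
; ToggleQuestion toggles the teacher or practice widget on the server and makes it block visibility traces, while HideQuestion hides meshes and student widget contents.
; Show/hide functions call client events that change the student widget or mesh visibility only without authority.
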(event `self.ReceiveTick`
  (params (DeltaSeconds :type "Float (single-precision)"))
  (bind _asumg_question_teacher (cast `/Game/_import/UI/UMG_QuestionTeacher` (`WidgetComponent.GetUserWidgetObject` (`self.QuestionTeacher`))))
  (`/Game/_import/UI/UMG_QuestionTeacher.SetTexts` _asumg_question_teacher (`self.Notice`) (`self.Question`) (`self.Answers`))
  (`/Game/_import/UI/UMG_QuestionTeacher.SetObject` _asumg_question_teacher self)
  (bind _asumg_question_practice (cast `/Game/_import/UI/UMG_QuestionPractice` (`WidgetComponent.GetUserWidgetObject` (`self.QuestionPractice`))))
  (`/Game/_import/UI/UMG_QuestionPractice.SetTexts` _asumg_question_practice (`self.Notice`) (`self.Question`) (`self.Answers`))
  (`/Game/_import/UI/UMG_QuestionPractice.SetObject` _asumg_question_practice self)
  (bind _asumg_question_student (cast `/Game/_import/UI/UMG_QuestionStudent` (`WidgetComponent.GetUserWidgetObject` (`self.QuestionStudent`))))
  (`/Game/_import/UI/UMG_QuestionStudent.SetTexts` _asumg_question_student (`self.Notice`) (`self.Question`) (`self.Answers`))
  (`/Game/_import/UI/UMG_QuestionStudent.SetObject` _asumg_question_student self))

(event `ShowHideNoticeClient`
  (params (NoticeShown :type Boolean))
  (`/Engine/EditorBlueprintResources/ActorMacros.Switch Has Authority`
    (:`Remote`
      (bind _asumg_question_student (cast `/Game/_import/UI/UMG_QuestionStudent` (`WidgetComponent.GetUserWidgetObject` (`self.QuestionStudent`))))
      (`/Game/_import/UI/UMG_QuestionStudent.ShowHideNotice` _asumg_question_student NoticeShown))))

(event `ShowHideObjectClient`
  (params (ObjectShown :type Boolean))
  (`/Engine/EditorBlueprintResources/ActorMacros.Switch Has Authority`
    (:`Remote`
      (for _array_element (`self.K2_GetComponentsByClass` "/Script/Engine.StaticMeshComponent")
        (`SceneComponent.SetVisibility` _array_element ObjectShown false)))))

(event `ShowHideQuestionClient`
  (params (QuestionShown :type Boolean))
  (`/Engine/EditorBlueprintResources/ActorMacros.Switch Has Authority`
    (:`Remote`
      (bind _asumg_question_student (cast `/Game/_import/UI/UMG_QuestionStudent` (`WidgetComponent.GetUserWidgetObject` (`self.QuestionStudent`))))
      (`/Game/_import/UI/UMG_QuestionStudent.ShowHideQuestion` _asumg_question_student QuestionShown))))

(fn `HideQuestion`
  (bind _questionstudent (`self.QuestionStudent`))
  ;[1 1 1] set question widget visible but hide buttons
  (`SceneComponent.SetVisibility` _questionstudent true false)
  (`PrimitiveComponent.SetCollisionResponseToChannel` _questionstudent "ECC_Visibility" "ECR_Block")
  (bind _asumg_question_student (cast `/Game/_import/UI/UMG_QuestionStudent` (`WidgetComponent.GetUserWidgetObject` _questionstudent)))
  (`/Game/_import/UI/UMG_QuestionStudent.HideAll` _asumg_question_student)
  ;[1 1 1] hide also all static mesh components
  (for _array_element (`self.K2_GetComponentsByClass` "/Script/Engine.StaticMeshComponent")
    (`SceneComponent.SetVisibility` _array_element false false)))

(fn `ShowHideNotice`
  (params (NoticeShown :type Boolean))
  (`self.ShowHideNoticeClient` NoticeShown))

(fn `ShowHideObject`
  (params (ObjectShown :type Boolean))
  (`self.ShowHideObjectClient` ObjectShown))

(fn `ShowHideQuestion`
  (params (QuestionShown :type Boolean))
  (`self.ShowHideQuestionClient` QuestionShown))

(fn `ToggleQuestion`
  (params (Server :type Boolean) (Practicing :type Boolean))
  (bind _questionpractice (`self.QuestionPractice`))
  (bind _questionteacher (`self.QuestionTeacher`))
  ;[1 1 1] check if teacher, practice or student and show depending widget and set response channel for trace
  (if Server
    (if Practicing
      (`SceneComponent.ToggleVisibility` _questionpractice false)
      (`PrimitiveComponent.SetCollisionResponseToChannel` _questionpractice "ECC_Visibility" "ECR_Block")
      (else
        (`SceneComponent.ToggleVisibility` _questionteacher false)
        (`PrimitiveComponent.SetCollisionResponseToChannel` _questionteacher "ECC_Visibility" "ECR_Block")))))

(fn `UserConstructionScript`)